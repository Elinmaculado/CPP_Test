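; Player pawn Blueprint that sets up Enhanced Input and handles pausing and the end screen, with no movement logic in its graphs.
; On controller change, it adds the IM_BaseGameMode mapping context for player controllers.
; IA_Pause toggles game pause, the cursor and a lazily created, reused WB_Pause widget.
; Destruction of the pawn is treated as death, showing WB_EndMenu and the cursor.
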(event `self.ReceiveControllerChanged`
  (params (OldController :type "Controller Object Reference") (NewController :type "Controller Object Reference"))
  ; Input actions
  (bind _asplayer_controller (cast `PlayerController` NewController))
  (message `EnhancedInputSubsystemInterface.AddMappingContext` (pcsubsystem `EnhancedInputLocalPlayerSubsystem` _asplayer_controller) "/Game/Input/IM_BaseGameMode.IM_BaseGameMode" 0 (struct)))

(event `EnhancedInput|/Game/Input/Inputs/IA_Pause`
  (params (ActionValue :type Boolean) (ElapsedSeconds :type "Float (double-precision)") (TriggeredSeconds :type "Float (double-precision)") (InputAction :type "InputAction Object Reference" :default "/Game/Input/Inputs/IA_Pause.IA_Pause"))
  ; Pause Input
  (:`Started`
    (`/Engine/EditorBlueprintResources/StandardMacros.IsValid` (`self.PauseMenu`)
      (:`Is Valid`
        _)
      (:`Is Not Valid`
        (bind _returnvalue (`|CreateWidget` "/Game/Blueprint/Widgets/WB_Pause.WB_Pause_C"))
        (set `self.PauseMenu` _returnvalue)))
    (if (`GameplayStatics.IsGamePaused`)
      (`Widget.RemoveFromParent` (`self.PauseMenu`))
      (`GameplayStatics.SetGamePaused` false)
      (set `PlayerController.bShowMouseCursor` false (`GameplayStatics.GetPlayerController` 0))
      (else
        (`UserWidget.AddToViewport` (`self.PauseMenu`) 0)
        (`GameplayStatics.SetGamePaused` true)
        (set `PlayerController.bShowMouseCursor` true (`GameplayStatics.GetPlayerController` 0))))))

(event `self.ReceiveDestroyed`
  ; Dead
  (bind _returnvalue (`|CreateWidget` "/Game/Blueprint/Widgets/WB_EndMenu.WB_EndMenu_C"))
  (`UserWidget.AddToViewport` _returnvalue 0)
  (set `PlayerController.bShowMouseCursor` true (`GameplayStatics.GetPlayerController` 0)))

(fn `UserConstructionScript`)